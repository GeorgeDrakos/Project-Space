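; Base enemy Blueprint that uses PawnSensing to detect the ThirdPersonCharacter player and chase it.
; Seeing the player triggers AI MoveTo toward that character, while hearing the player only prints a debug message.
; Every Tick, the enemy also emits noise at its own location through both PawnNoiseEmitter MakeNoise and an AI perception ReportNoiseEvent.
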(event EventBeginPlay)

(event Collision|EventActorBeginOverlap
  (params (OtherActor :type Actor%20Object%20Reference)))

(event EventTick
  (params (DeltaSeconds :type Float%20%28single-precision%29))
  (Class|PawnNoiseEmitterComponent|MakeNoise (Variables|Default|GetPawnNoiseEmitter) self 1.0 (Transformation|GetActorLocation))
  (Class|AISenseHearing|ReportNoiseEvent (Transformation|GetActorLocation) 1.0 self 0.0 "None"))

(event OnSeePawn(PawnSensing)
  (params (Pawn :type Pawn%20Object%20Reference))
  ;[1 1 1] AI See and Hear
  (bind _asthird_person_character (Utilities|Casting|CastToThirdPersonCharacter Pawn))
  (AI|AIMoveTo self (Transformation|GetActorLocation _asthird_person_character) _asthird_person_character 5.0 false))

(event OnHearNoise(PawnSensing)
  (params (Instigator :type Pawn%20Object%20Reference) (Location :type Vector%20%28by%20ref%29 :default "0, 0, 0") (Volume :type Float%20%28single-precision%29))
  ;[1 1 1] AI See and Hear
  (Utilities|Casting|CastToThirdPersonCharacter Instigator)
  (Development|PrintText "I can hear the player"))

(fn ConstructionScript)